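; BP_PriorityLayer is a custom UI layer that hides all other layers it receives when a widget is pushed to it.
; On push, it saves each other layer's visibility in the LayersVisibility map, then collapses that layer.
; On pop, it restores the saved visibility for layers found in the map, then clears it.
; The layer's own push and pop events only call the parent implementation.
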(event `self.OnWidgetPopped`
  (params (widget :type "UserWidget Object Reference"))
  ;[1 1 1 1 12] Custom layers allow defining behaviour when popping or pushing widgets, for example if a widget is of a certain type play an animation
  (`parent.OnWidgetPopped` widget))

(event `self.OnWidgetPushed`
  (params (widget :type "UserWidget Object Reference"))
  ;[1 1 1 1 12] Custom layers allow defining behaviour when popping or pushing widgets, for example if a widget is of a certain type play an animation
  (`parent.OnWidgetPushed` widget))

(event `self.OnWidgetPushedOthers`
  (params (otherLayers :type "Array of LayerUI Object Reference (by ref)"))
  ;[1 1 1 1 16] By creating functionality here you can define what happens to other layers when you push a widget to a layer of this type of layer.For example, here when a widget is pushed to the priority layer, the visibility of all the other layers is saved and restored when a widget is popped.
  (for _array_element otherLayers
    (`BlueprintMapLibrary.Map_Add` (`self.LayersVisibility`) _array_element (`self.GetVisibilityOfLayer` _array_element))
    (`self.SetVisibilityOfLayer` _array_element "Collapsed")))

(event `self.OnWidgetPoppedOthers`
  (params (otherLayers :type "Array of LayerUI Object Reference (by ref)"))
  ;[1 1 1 1 16] By creating functionality here you can define what happens to other layers when you push a widget to a layer of this type of layer.For example, here when a widget is pushed to the priority layer, the visibility of all the other layers is saved and restored when a widget is popped.
  (for _array_element otherLayers
    (bind (_value _returnvalue) (`BlueprintMapLibrary.Map_Find` (`self.LayersVisibility`) _array_element))
    (if _returnvalue
      (`self.SetVisibilityOfLayer` _array_element _value)))
  (`BlueprintMapLibrary.Map_Clear` (`self.LayersVisibility`)))